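; Boss enemy that patrols along the X axis, deals delayed contact damage to BP_Paladin and creates a boss health bar widget on BeginPlay.
; Each Tick moves it forward, using downward traces at the capsule edges to turn around at ledges.
; A sphere trace plus an eye line-of-sight trace detects the Paladin, switching ledge turns to stops.
; It destroys itself once health is depleted; Shooting and ItsMele are never called here.
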(event OnComponentHit(CapsuleComponent)
  (params (HitComponent :type Primitive%20Component%20Object%20Reference) (OtherActor :type Actor%20Object%20Reference) (OtherComp :type Primitive%20Component%20Object%20Reference) (NormalImpulse :type Vector :default "0, 0, 0") (Hit :type Hit%20Result%20Structure%20%28by%20ref%29))
  ;[1 1 1] Boss Attack
  (if (> (Variables|Default|GetBossEnemyHealth) 0.0)
    (Variables|Default|Setspeed 0.0)
    (bind _asbp_paladin (Utilities|Casting|CastToBP_Paladin OtherActor))
    (Utilities|FlowControl|Delay 0.5)
    (Default|TakeDamage _asbp_paladin (Variables|Default|GetBossDamage))
    (else
      (Actor|DestroyActor))))

(event EventTick
  (params (DeltaSeconds :type Float%20%28single-precision%29))
  ;[1 1 1] Boss Movement and Detection
  (if (> (Variables|Default|GetBossEnemyHealth) 0.0)
    (bind (_detected _character) (CallFunction|CheckCharacter))
    (if _detected
      (bind _detected_2 (CallFunction|CheckVision _character))
      (if _detected_2
        ;[1 1 1] Boss Check Limits
        (CallFunction|GetDirection)
        (bind _output_get (CallFunction|ChecklimitsrightStop))
        (bind _output_get_2 (CallFunction|Checklimitsleftstop))
        (if (or _output_get _output_get_2)
          (Variables|Default|Setspeed 0.0)
          (else
            (Pawn|Input|AddMovementInput (Math|Vector|GetForwardVector (Math|Rotator|MakeRotator 0.0 0.0 (.yaw (Pawn|GetControlRotation :!class /Script/Engine.Pawn)))) 1.0 false)))
        (else
          (CallFunction|Checklimitsright :!label _label)
          (CallFunction|Checklimitsleft)
          (Pawn|Input|AddMovementInput (Math|Vector|GetForwardVector (Math|Rotator|MakeRotator 0.0 0.0 (.yaw (Pawn|GetControlRotation :!class /Script/Engine.Pawn)))) 1.0 false)))
      (else
        (goto _label)))
    (else
      (Actor|DestroyActor))))

(event EventBeginPlay
  ;[1 1 1] Boss Health bar
  (bind _returnvalue (UserInterface|CreateWidget "/Game/MyContent/UI/WBP_BossHealth.WBP_BossHealth_C" (Game|GetPlayerController 0) 0))
  (Variables|/Game/MyContent/UI/WBP_BossHealth.WBP_BossHealth_C|SetBoss _returnvalue 0)
  (UserInterface|Viewport|AddtoViewport _returnvalue 0))

(fn ConstructionScript)

(fn Checklimitsright
  (bind _capsulecomponent (Variables|Collision|GetCapsuleComponent))
  (bind (_origin _boxextent) (Collision|GetComponentBounds _capsulecomponent))
  (bind _returnvalue (+ (.x _origin) (.x _boxextent)))
  (bind _returnvalue_2 (- (.z _origin) (.z _boxextent)))
  (bind _returnvalue_3 (Collision|LineTraceByChannel (Math|Vector|MakeVector _returnvalue (.y _origin) _returnvalue_2) (Math|Vector|MakeVector _returnvalue (.y _origin) (- _returnvalue_2 5e+01)) "TraceTypeQuery1" false 0 "ForOneFrame"))
  (if (not _returnvalue_3)
    (Variables|Default|Setspeed (* (Variables|Default|Getspeed) -1.0))
    (Transformation|SetActorRotation "0.000000,180.000000,0.000000")
    (Variables|Default|SetItsrotateted true)))

(fn Checklimitsleft
  (bind _capsulecomponent (Variables|Collision|GetCapsuleComponent))
  (bind (_origin _boxextent) (Collision|GetComponentBounds _capsulecomponent))
  (bind _returnvalue (- (.z _origin) (.z _boxextent)))
  (bind _returnvalue_2 (- (.x _origin) (.x _boxextent)))
  (bind _returnvalue_3 (Collision|LineTraceByChannel (Math|Vector|MakeVector _returnvalue_2 (.y _origin) _returnvalue) (Math|Vector|MakeVector _returnvalue_2 (.y _origin) (- _returnvalue 5e+01)) "TraceTypeQuery1" false 0 "ForOneFrame"))
  (if (not _returnvalue_3)
    (Variables|Default|Setspeed (* (Variables|Default|Getspeed) -1.0))
    (Transformation|SetActorRotation "0, 0, 0")
    (Variables|Default|SetItsrotateted false)))

(fn CheckCharacter
  (bind _returnvalue (Transformation|GetActorLocation))
  (bind (_outhits _returnvalue_2) (Collision|MultiSphereTraceByChannel _returnvalue _returnvalue 5e+02 "TraceTypeQuery1" false 0 "ForOneFrame" false))
  (bind _array_element (Utilities|Array|ForEachLoopwithBreak _outhits)
    (:LoopBody
      (bind _asbp_paladin (Utilities|Casting|CastToBP_Paladin (.HitActor (Collision|BreakHitResult _array_element))))
      (return _returnvalue_2 _asbp_paladin))
    (:Completed
      (return false 0))))

(fn CheckVision
  (params (Character :type BP%20Paladin%20Object%20Reference))
  (Utilities|IsValid Character
    (:Is%20Valid
      (bind _outhit (Collision|LineTraceByChannel (Transformation|GetWorldLocation (Variables|Default|GetEyes)) (Transformation|GetActorLocation Character) "TraceTypeQuery1" false 0 "ForOneFrame" false))
      (Utilities|Casting|CastToBP_Paladin (.HitActor (Collision|BreakHitResult _outhit))
        (:then
          (return true))
        (:CastFailed
          (return false))))))

(fn Shooting
  (params (Character :type BP%20Third%20Person%20Character%20Object%20Reference))
  (Game|SpawnActorfromClass "/Game/MyContent/Blueprints/Proyectile/Bullet.Bullet_C" (Transformation|GetWorldTransform (Variables|Default|GetEyes)) "Undefined" "OverrideRootScale" 0 Character "NewEnumerator2" 0))

(fn GetDirection
  (Utilities|IsValid (Variables|Default|GetCharacterReference)
    (:Is%20Valid
      (Variables|Default|SetDirection (Math|Vector|Normalize (- (Transformation|GetWorldLocation (Variables|Character|GetMesh)) (Transformation|GetActorLocation)))))))

(fn ChecklimitsrightStop
  (bind _capsulecomponent (Variables|Collision|GetCapsuleComponent))
  (bind (_origin _boxextent) (Collision|GetComponentBounds _capsulecomponent))
  (bind _returnvalue (+ (.x _origin) (.x _boxextent)))
  (bind _returnvalue_2 (- (.z _origin) (.z _boxextent)))
  (bind _returnvalue_3 (Collision|LineTraceByChannel (Math|Vector|MakeVector _returnvalue (.y _origin) _returnvalue_2) (Math|Vector|MakeVector _returnvalue (.y _origin) (- _returnvalue_2 5e+01)) "TraceTypeQuery1" false 0 "ForOneFrame"))
  (if _returnvalue_3
    (bind _output_get (Variables|Default|Setstop false))
    (return _output_get)
    (elif (Variables|Default|GetItsrotateted)
      (bind _output_get_2 (Variables|Default|Setstop false))
      (return _output_get_2)
      (else
        (bind _output_get_3 (Variables|Default|Setstop true))
        (return _output_get_3)))))

(fn Checklimitsleftstop
  (bind _capsulecomponent (Variables|Collision|GetCapsuleComponent))
  (bind (_origin _boxextent) (Collision|GetComponentBounds _capsulecomponent))
  (bind _returnvalue (- (.z _origin) (.z _boxextent)))
  (bind _returnvalue_2 (- (.x _origin) (.x _boxextent)))
  (bind _returnvalue_3 (Collision|LineTraceByChannel (Math|Vector|MakeVector _returnvalue_2 (.y _origin) _returnvalue) (Math|Vector|MakeVector _returnvalue_2 (.y _origin) (- _returnvalue 5e+01)) "TraceTypeQuery1" false 0 "ForOneFrame"))
  (if _returnvalue_3
    (bind _output_get (Variables|Default|Setstop false))
    (return _output_get)
    (elif (Variables|Default|GetItsrotateted)
      (bind _output_get_2 (Variables|Default|Setstop true))
      (return _output_get_2)
      (else
        (bind _output_get_3 (Variables|Default|Setstop false))
        (return _output_get_3)))))

(fn ItsMele
  (bind _returnvalue (Transformation|GetActorLocation))
  (bind _outhit (Collision|LineTraceByChannel _returnvalue _returnvalue "TraceTypeQuery1" false 0 "None")))

(fn EnemyBossTakeDamage
  (params (Damage :type Float%20%28double-precision%29))
  (Variables|Default|SetBossEnemyHealth (- (Variables|Default|GetBossEnemyHealth) Damage)))