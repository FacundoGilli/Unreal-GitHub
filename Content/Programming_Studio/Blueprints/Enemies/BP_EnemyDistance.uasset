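; Ranged enemy that patrols along platforms and fires projectiles at BP_Paladin when it is nearby and visible.
; Each Tick, a sphere trace detects the Paladin and an Eyes line trace confirms sight before spawning a Bullet, paced by a Delay.
; Otherwise it walks forward, using downward traces at both capsule sides to turn around at ledges.
; EnemyDistanceTakeDamage lowers health, and Tick destroys the actor once it runs out.
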(event EventTick
  (params (DeltaSeconds :type Float%20%28single-precision%29))
  ;[1 1 1] Enemy Checking Character and vision
  (if (> (Variables|Default|GetDistanceEnemyHealth) 0.0)
    (bind (_detected _character) (CallFunction|CheckCharacter))
    (if _detected
      (bind _detected_2 (CallFunction|CheckVision _character))
      (if _detected_2
        ;[1 1 1] Enemy Shoot
        (Utilities|FlowControl|Delay 1.5)
        (CallFunction|Shooting _character)
        (else
          ;[1 1 1] Enemy Movement
          (CallFunction|Checklimitsright :!label _label)
          (CallFunction|Checklimitsleft)
          (Pawn|Input|AddMovementInput (Math|Vector|GetForwardVector (Math|Rotator|MakeRotator 0.0 0.0 (.yaw (Pawn|GetControlRotation :!class /Script/Engine.Pawn)))) 1.0 false)))
      (else
        (goto _label)))
    (else
      (Actor|DestroyActor))))

(fn ConstructionScript)

(fn Checklimitsright
  (bind _capsulecomponent (Variables|Collision|GetCapsuleComponent))
  (bind (_origin _boxextent) (Collision|GetComponentBounds _capsulecomponent))
  (bind _returnvalue (+ (.x _origin) (.x _boxextent)))
  (bind _returnvalue_2 (- (.z _origin) (.z _boxextent)))
  (bind _returnvalue_3 (Collision|LineTraceByChannel (Math|Vector|MakeVector _returnvalue (.y _origin) _returnvalue_2) (Math|Vector|MakeVector _returnvalue (.y _origin) (- _returnvalue_2 5e+01)) "TraceTypeQuery1" false 0 "ForOneFrame"))
  (if (not _returnvalue_3)
    (Variables|Default|Setspeed (* (Variables|Default|Getspeed) -1.0))
    (Transformation|SetActorRotation "0.000000,180.000000,0.000000")))

(fn Checklimitsleft
  (bind _capsulecomponent (Variables|Collision|GetCapsuleComponent))
  (bind (_origin _boxextent) (Collision|GetComponentBounds _capsulecomponent))
  (bind _returnvalue (- (.z _origin) (.z _boxextent)))
  (bind _returnvalue_2 (- (.x _origin) (.x _boxextent)))
  (bind _returnvalue_3 (Collision|LineTraceByChannel (Math|Vector|MakeVector _returnvalue_2 (.y _origin) _returnvalue) (Math|Vector|MakeVector _returnvalue_2 (.y _origin) (- _returnvalue 5e+01)) "TraceTypeQuery1" false 0 "ForOneFrame"))
  (if (not _returnvalue_3)
    (Variables|Default|Setspeed (* (Variables|Default|Getspeed) -1.0))
    (Transformation|SetActorRotation "0, 0, 0")))

(fn CheckCharacter
  (bind _returnvalue (Transformation|GetActorLocation))
  (bind _outhits (Collision|MultiSphereTraceByChannel _returnvalue _returnvalue 5e+02 "TraceTypeQuery1" false 0 "ForOneFrame" false))
  (bind _array_element (Utilities|Array|ForEachLoopwithBreak _outhits)
    (:LoopBody
      (bind _asbp_paladin (Utilities|Casting|CastToBP_Paladin (.HitActor (Collision|BreakHitResult _array_element))))
      (return true _asbp_paladin))
    (:Completed
      (return false 0))))

(fn CheckVision
  (params (Character :type BP%20Paladin%20Object%20Reference))
  (Utilities|IsValid Character
    (:Is%20Valid
      (bind _outhit (Collision|LineTraceByChannel (Transformation|GetWorldLocation (Variables|Default|GetEyes)) (Transformation|GetActorLocation Character) "TraceTypeQuery1" false 0 "ForOneFrame" false))
      (Utilities|Casting|CastToBP_Paladin (.HitActor (Collision|BreakHitResult _outhit))
        (:then
          (return true))
        (:CastFailed
          (return false))))))

(fn Shooting
  (params (Character :type BP%20Paladin%20Object%20Reference))
  (Game|SpawnActorfromClass "/Game/MyContent/Blueprints/Proyectile/Bullet.Bullet_C" (Transformation|GetWorldTransform (Variables|Default|GetEyes)) "Undefined" "OverrideRootScale" 0 Character "NewEnumerator2" 0))

(fn EnemyDistanceTakeDamage
  (params (Damage :type Float%20%28double-precision%29))
  (Variables|Default|SetDistanceEnemyHealth (- (Variables|Default|GetDistanceEnemyHealth) Damage)))