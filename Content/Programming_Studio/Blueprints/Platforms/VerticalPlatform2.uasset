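; Vertical moving platform that ping-pongs along Z between its starting height and a point Distance above it.
; BeginPlay stores the start location, and each Tick calls MoveDown, which subtracts Speed times delta seconds from Z.
; PingPongCondition then checks whether Z is at or beyond either limit, and Tick negates Speed if so, without clamping the position.
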(event EventBeginPlay
  (Variables|Default|SetInitpos (Transformation|GetActorLocation)))

(event Collision|EventActorBeginOverlap
  (params (OtherActor :type Actor%20Object%20Reference)))

(event EventTick
  (params (DeltaSeconds :type Float%20%28single-precision%29))
  (CallFunction|MoveDown)
  (if (CallFunction|PingPongCondition)
    (Variables|Default|SetSpeed (* (Variables|Default|GetSpeed) -1.0))))

(fn ConstructionScript)

(fn MoveDown
  (bind _returnvalue (Transformation|GetActorLocation))
  (Transformation|SetActorLocation (Math|Vector|MakeVector (.x _returnvalue) (.y _returnvalue) (- (.z _returnvalue) (* (Utilities|Time|GetWorldDeltaSeconds) (Variables|Default|GetSpeed)))) false false))

(fn PingPongCondition
  (return (or (<= (+ (.z (Variables|Default|GetInitpos)) (Variables|Default|GetDistance)) (.z (Transformation|GetActorLocation))) (>= (.z (Variables|Default|GetInitpos)) (.z (Transformation|GetActorLocation))))))