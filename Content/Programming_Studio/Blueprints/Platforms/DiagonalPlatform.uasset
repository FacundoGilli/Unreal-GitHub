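; A moving platform Blueprint that travels back and forth along a diagonal in the X-Z plane.
; BeginPlay stores the starting location, and each Tick shifts the actor equally in X and Z by Speed scaled by delta time.
; Speed flips sign whenever X is at or beyond either the start or start plus Distance, with no position clamping.
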(event EventBeginPlay
  (Variables|Default|SetInitialpos (Transformation|GetActorLocation)))

(event Collision|EventActorBeginOverlap
  (params (OtherActor :type Actor%20Object%20Reference)))

(event EventTick
  (params (DeltaSeconds :type Float%20%28single-precision%29))
  (CallFunction|MoveDiagonal)
  (if (CallFunction|PingPongDiagonalCondition)
    (Variables|Default|SetSpeed (* (Variables|Default|GetSpeed) -1.0))))

(fn ConstructionScript)

(fn MoveDiagonal
  (bind _returnvalue (Transformation|GetActorLocation))
  (Transformation|SetActorLocation (Math|Vector|MakeVector (+ (* (Utilities|Time|GetWorldDeltaSeconds) (Variables|Default|GetSpeed)) (.x _returnvalue)) (.y _returnvalue) (+ (.z _returnvalue) (* (Utilities|Time|GetWorldDeltaSeconds) (Variables|Default|GetSpeed)))) false false))

(fn PingPongDiagonalCondition
  (return (or (<= (+ (.x (Variables|Default|GetInitialpos)) (Variables|Default|GetDistance)) (.x (Transformation|GetActorLocation))) (>= (.x (Variables|Default|GetInitialpos)) (.x (Transformation|GetActorLocation))))))