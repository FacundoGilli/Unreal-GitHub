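; Operadores is an Actor sandbox of exercises on Blueprint operators and control flow, printing results as strings.
; Its EventGraph holds disconnected snippets for comparisons, integer math, branches, switches, loops, float-accumulator timers and X-axis movement; none runs, as all events are empty.
; Three standalone functions add two numbers, sum the min and max of four, and scan a float array for an extreme.
; The array's minimum branch assigns 0.0 instead of the smaller element.
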(event EventBeginPlay)

(event Collision|EventActorBeginOverlap
  (params (OtherActor :type Actor%20Object%20Reference)))

(event EventTick
  (params (DeltaSeconds :type Float%20%28single-precision%29)))

(fn ConstructionScript)

(fn AddTwoNumbers
  (params (First%20Number :type Float%20%28double-precision%29) (Second%20Number :type Float%20%28double-precision%29))
  (return (+ First%20Number Second%20Number)))

(fn Ejercicio1
  (params (Numero%201 :type Float%20%28double-precision%29) (Numer%202 :type Float%20%28double-precision%29) (Numero%203 :type Float%20%28double-precision%29) (Numero%204 :type Float%20%28double-precision%29))
  (return (+ (Math|Float|Min(Float) Numero%201 Numer%202 Numero%203 Numero%204) (Math|Float|Max(Float) Numero%201 Numer%202 Numero%203 Numero%204))))

(fn Ejercicio2
  (params (FloatArray :type Array%20of%20Floats%20%28double-precision%29) (Max :type Boolean))
  (LocalVariables|SetFloatToCompare (Utilities|Array|Get(acopy) FloatArray))
  (if Max
    (for _array_element FloatArray
      (if (> _array_element (LocalVariables|GetFloatToCompare))
        (LocalVariables|SetFloatToCompare _array_element)))
    (return (LocalVariables|GetFloatToCompare))
    (else
      (for _array_element_2 FloatArray
        (if (< _array_element_2 (LocalVariables|GetFloatToCompare))
          (LocalVariables|SetFloatToCompare 0.0)))
      (return (LocalVariables|GetFloatToCompare)))))