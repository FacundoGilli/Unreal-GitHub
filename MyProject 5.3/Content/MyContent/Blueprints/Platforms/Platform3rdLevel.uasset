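; Platform Blueprint that opens ThirdLevel from Tick when the FromSweep value of its Box overlap event is true.
; The Box overlap casts to BP_Paladin but runs nothing afterward, so the cast does not gate the level change.
; Movement offsets the actor along Direction at a frame-scaled Speed, and CheckLimits detects proximity to either travel endpoint.
; Neither function is called in this Blueprint.
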(event OnComponentBeginOverlap(Box)
  (params (OverlappedComponent :type Primitive%20Component%20Object%20Reference) (OtherActor :type Actor%20Object%20Reference) (OtherComp :type Primitive%20Component%20Object%20Reference) (OtherBodyIndex :type Integer) (bFromSweep :type Boolean) (SweepResult :type Hit%20Result%20Structure%20%28by%20ref%29))
  (Utilities|Casting|CastToBP_Paladin OtherActor))

(event EventBeginPlay)

(event Collision|EventActorBeginOverlap
  (params (OtherActor :type Actor%20Object%20Reference)))

(event EventTick
  (params (DeltaSeconds :type Float%20%28single-precision%29))
  (if (stale OnComponentBeginOverlap(Box) bFromSweep)
    (Game|OpenLevel(byName) "ThirdLevel")))

(fn ConstructionScript)

(fn Movement
  (Transformation|SetActorLocation (+ (Transformation|GetActorLocation) (* (Math|Vector|Normalize (Variables|Default|GetDirection)) (* (Variables|Default|GetSpeed) (Utilities|Time|GetWorldDeltaSeconds)))) false false))

(fn CheckLimits
  (if (or (<= (Math|Vector|Distance(Vector) (Variables|Default|GetInicpos) (Transformation|GetActorLocation)) 1e+01) (<= (Math|Vector|Distance(Vector) (+ (Variables|Default|GetInicpos) (* (Math|Vector|Normalize (Variables|Default|GetDirection)) (Variables|Default|GetDistance))) (Transformation|GetActorLocation)) 1e+01))
    (return true)
    (else
      (return false))))