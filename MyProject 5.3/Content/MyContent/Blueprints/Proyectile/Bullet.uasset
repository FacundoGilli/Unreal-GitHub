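; Bullet projectile actor that targets a referenced character and damages BP_Paladin on overlap, destroying itself whether or not the Paladin is blocking.
; Aimed bullets compute a direction once at spawn, while Homing bullets recompute it each Tick and move by Speed without sweep.
; Blocking negates the damage.
; A delayed self-destruct for Homing bullets sits behind a constant-false branch, and no movement for Aimed bullets appears in this graph.
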(event EventBeginPlay
  ;[1 1 1] Bullet Destroy
  (switch Utilities|FlowControl|Switch|SwitchonTypeOfBullet (Variables|Default|GetBulletType)
    (:NewEnumerator1
      (CallFunction|GetDirection))
    (:NewEnumerator2
      (if (not true)
        (Timeline|DrestoyActorDelay Play
          (:Finished
            (Utilities|IsValid self
              (:Is%20Valid
                (Actor|DestroyActor)))))))))

(event EventTick
  (params (DeltaSeconds :type Float%20%28single-precision%29))
  ;[1 1 1] Bullet Following
  (if (Utilities|Enum|Equal(Enum) (Variables|Default|GetBulletType) "NewEnumerator2")
    (CallFunction|GetDirection)
    (Transformation|SetActorLocation (+ (Transformation|GetActorLocation) (* (Variables|Default|GetDirection) (* DeltaSeconds (Variables|Default|GetSpeed)))) false false)))

(event Collision|EventActorBeginOverlap
  (params (OtherActor :type Actor%20Object%20Reference))
  ;[1 1 1] Bullet Damage
  (bind _asbp_paladin (Utilities|Casting|CastToBP_Paladin OtherActor))
  (if (Variables|/Game/MyContent/Blueprints/Characters/BP_Paladin.BP_Paladin_C|GetIs%20Blocking _asbp_paladin)
    (Actor|DestroyActor)
    (else
      (Default|TakeDamage _asbp_paladin (Variables|Default|GetBulletDamage))
      (Actor|DestroyActor))))

(fn ConstructionScript)

(fn GetDirection
  (bind _characterreference (Variables|Default|GetCharacterReference))
  (Utilities|IsValid _characterreference
    (:Is%20Valid
      (Variables|Default|SetDirection (Math|Vector|Normalize (- (Transformation|GetActorLocation _characterreference) (Transformation|GetActorLocation)))))))